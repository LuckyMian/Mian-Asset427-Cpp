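; Spline actor that builds a chain of spline meshes along an optionally looped spline, with animated masking and scale.
; Construction script segments by fixed distance or spline point, using either scaled-direction or true spline tangents.
; Each segment's dynamic material receives its fraction of total length, so UVs can run across the whole spline, plus speed and tiling.
; Custom events toggle timelines that drive start/end mask parameters and pulse mesh thickness.
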(event `MeshScale`
  (bind _mesharray (`self.MeshArray`))
  (bind _dynamicscalemesh (`self.DynamicScaleMesh`))
  (`/Engine/EditorBlueprintResources/StandardMacros.FlipFlop`
    (:`A`
      (bind (_direction _newtrack_0) (`Timeline|Timeline_4` :!label _label)
        (:`Update`
          (bind _returnvalue (`KismetMathLibrary.Lerp` _dynamicscalemesh (* _dynamicscalemesh 1.5) _newtrack_0))
          (`SplineMeshComponent.SetStartScale` _mesharray (`KismetMathLibrary.MakeVector2D` _returnvalue _returnvalue) true)
          (`SplineMeshComponent.SetEndScale` _mesharray (`KismetMathLibrary.MakeVector2D` _returnvalue _returnvalue) true))))
    (:`B`
      (goto _label :!via `Reverse`))))

(event `StartMask2`
  (bind _dynamicmaterialarray (`self.DynamicMaterialArray`))
  (`/Engine/EditorBlueprintResources/StandardMacros.FlipFlop`
    (:`A`
      (bind (_direction _newtrack_0) (`Timeline|Timeline_2` :!label _label_2)
        (:`Update`
          (bind _returnvalue (`KismetMathLibrary.Lerp` 0.0 1.0 _newtrack_0))
          (`MaterialInstanceDynamic.SetScalarParameterValue` _dynamicmaterialarray "BPEndMask" _returnvalue)
          (`MaterialInstanceDynamic.SetScalarParameterValue` _dynamicmaterialarray "BPStartMask" _returnvalue))))
    (:`B`
      (goto _label_2 :!via `Reverse`))))

(event `StartMask`
  (bind _dynamicmaterialarray (`self.DynamicMaterialArray`))
  (`/Engine/EditorBlueprintResources/StandardMacros.DoOnce` false :!label _label_3
    (:`Completed`
      (`/Engine/EditorBlueprintResources/StandardMacros.FlipFlop`
        (:`A`
          (bind (_direction _newtrack_0) (`Timeline|Timeline_0` :!via `PlayFromStart`)
            (:`Update`
              (`MaterialInstanceDynamic.SetScalarParameterValue` _dynamicmaterialarray "BPEndMask" 1.0)
              (`MaterialInstanceDynamic.SetScalarParameterValue` _dynamicmaterialarray "BPStartMask" (`KismetMathLibrary.Lerp` 0.0 1.0 _newtrack_0)))
            (:`Finished`
              (goto _label_3 :!via `Reset`))))
        (:`B`
          (bind (_direction_2 _newtrack_0_2) (`Timeline|Timeline_1` :!via `PlayFromStart`)
            (:`Update`
              (`MaterialInstanceDynamic.SetScalarParameterValue` _dynamicmaterialarray "BPEndMask" (`KismetMathLibrary.Lerp` 1.0 0.0 _newtrack_0_2)))
            (:`Finished`
              (goto _label_3 :!via `Reset`))))))))

(fn `BPCommunicationMaterialUV`
  (params (FirstSegmentLength :type "Float (double-precision)") (SecondSegmentLength :type "Float (double-precision)") (TotalLenght :type "Float (double-precision)") (DynamicMaterial :type "MaterialInstanceDynamic Object Reference"))
  (bind (_returnvalue_x _returnvalue_y _returnvalue_z) (`KismetMathLibrary.BreakVector` (- (`KismetMathLibrary.MakeVector` FirstSegmentLength SecondSegmentLength TotalLenght) 0.0)))
  (`MaterialInstanceDynamic.SetScalarParameterValue` DynamicMaterial "BPLineMutiply" (/ (- _returnvalue_y _returnvalue_x) _returnvalue_z))
  (`MaterialInstanceDynamic.SetScalarParameterValue` DynamicMaterial "BPLineMove" (- 0.0 (/ _returnvalue_x _returnvalue_z))))

(fn `UserConstructionScript`
  (bind _dynamicscalemesh (`self.DynamicScaleMesh`))
  (bind _spline (`self.Spline`))
  (bind _tangentscale_type1_3 (`self.TangentScale(Type1 3`))
  (bind _tangentscale_type1_3_2 (`self.TangentScale(Type1 3`))
  (bind _dynamicscalemesh_2 (`self.DynamicScaleMesh`))
  (bind _tangentscale_type1_3_3 (`self.TangentScale(Type1 3`))
  (bind _dynamicscalemesh_3 (`self.DynamicScaleMesh`))
  (bind _dynamicscalemesh_4 (`self.DynamicScaleMesh`))
  (bind _dynamicmaterial (`self.DynamicMaterial`))
  (bind _dynamicscalemesh_5 (`self.DynamicScaleMesh`))
  (bind _dynamicmaterial_2 (`self.DynamicMaterial`))
  (bind _dynamicmaterial_3 (`self.DynamicMaterial`))
  (bind _spline_2 (`self.Spline`))
  (bind _spline_3 (`self.Spline`))
  (bind _dynamicscalemesh_6 (`self.DynamicScaleMesh`))
  (bind _meshdistancescale_type1 (`self.MeshDistanceScale(Type1`))
  (bind _returnvalue (`SplineComponent.GetSplineLength` (`self.Spline`)))
  (bind _returnvalue_2 (`SplineComponent.GetNumberOfSplinePoints` _spline_3))
  (bind _returnvalue_3 (`SplineComponent.GetSplineLength` (`self.Spline`)))
  (bind _returnvalue_4 (`KismetMathLibrary.SelectInt` (+ _returnvalue_2 1) _returnvalue_2 (`self.SplineLoop`)))
  (bind _returnvalue_5 (`SplineComponent.GetDistanceAlongSplineAtSplinePoint` _spline_3 (- _returnvalue_4 1)))
  (bind _returnvalue_6 (* (`KismetMathLibrary.Conv_IntToDouble` (`KismetMathLibrary.FCeil` (/ _returnvalue_3 (`self.DynamicScaleMesh`)))) 0.01))
  (bind _returnvalue_7 (* (`KismetMathLibrary.Conv_IntToDouble` (`KismetMathLibrary.FCeil` (/ _returnvalue (`self.DynamicScaleMesh`)))) 0.01))
  (bind _returnvalue_8 (* (/ _returnvalue_5 (`self.DynamicScaleMesh`)) 0.01))
  (`SplineComponent.SetClosedLoop` (`self.Spline`) (`self.SplineLoop`) true)
  (switch `/Game/AdvancedSplineMeshAnalysisTool/Blueprints/BP_SplineMeshType_Enum` (`self.SplineMeshType`)
    (:`NewEnumerator0`
      (for _index (range (`.ReturnValue` (`KismetMathLibrary.FMod` (`SplineComponent.GetSplineLength` (`self.Spline`)) (`self.MeshDistanceScale(Type1`))))
        (bind _returnvalue_9 (`AddComponent|NODE_AddSplineMeshComponent-3` :`bManualAttachment` true))
        (`SplineMeshComponent.SetSplineUpDir` _returnvalue_9 (`self.In Spline Up Dir`) true)
        (`StaticMeshComponent.SetStaticMesh` _returnvalue_9 (`self.MeshInstance`))
        (`SplineMeshComponent.SetStartScale` _returnvalue_9 (`KismetMathLibrary.MakeVector2D` _dynamicscalemesh_2 _dynamicscalemesh_2) true)
        (`SplineMeshComponent.SetEndScale` _returnvalue_9 (`KismetMathLibrary.MakeVector2D` _dynamicscalemesh_2 _dynamicscalemesh_2) true)
        (bind _output_get (set `self.SplineMeshArray` _returnvalue_9))
        (`KismetArrayLibrary.Array_Add` (`self.MeshArray`) _output_get)
        (`SplineMeshComponent.SetStartScale` _returnvalue_9 (`KismetMathLibrary.MakeVector2D` _dynamicscalemesh _dynamicscalemesh) true)
        (`SplineMeshComponent.SetEndScale` _returnvalue_9 (`KismetMathLibrary.MakeVector2D` _dynamicscalemesh _dynamicscalemesh) true)
        (bind _returnvalue_10 (`PrimitiveComponent.CreateDynamicMaterialInstance` _returnvalue_9 0 (`self.MaterialInstance`) "None"))
        (bind _output_get_2 (set `self.DynamicMaterial` _returnvalue_10))
        (`KismetArrayLibrary.Array_Add` (`self.DynamicMaterialArray`) _output_get_2)
        (`PrimitiveComponent.SetMaterial` _returnvalue_9 0 _returnvalue_10)
        (bind _returnvalue_11 (* _index _meshdistancescale_type1))
        (bind _returnvalue_12 (+ _returnvalue_11 _meshdistancescale_type1))
        ;[0 1 0.491] SplineMeshTypeOne(For tangents that do not fully fit the spline, mesh is generated according to the distance, and the tangent mode is generated according to the direction. Tangent scaling can be modified
        (`SplineMeshComponent.SetStartAndEnd` _returnvalue_9 (`SplineComponent.GetLocationAtDistanceAlongSpline` _spline _returnvalue_11 "World") (* (`SplineComponent.GetDirectionAtDistanceAlongSpline` _spline _returnvalue_11 "World") _tangentscale_type1_3_2) (`SplineComponent.GetLocationAtDistanceAlongSpline` _spline _returnvalue_12 "World") (* (`SplineComponent.GetDirectionAtDistanceAlongSpline` _spline _returnvalue_12 "World") _tangentscale_type1_3_2) true)
        (`self.BPCommunicationMaterialUV` _returnvalue_11 _returnvalue_12 _returnvalue_3 (`self.DynamicMaterial`)) ; Communication module with material
        (`MaterialInstanceDynamic.SetScalarParameterValue` _dynamicmaterial_2 "BPSpeed" (`self.Speed`))
        (if (`self.TextureLoop`)
          (`MaterialInstanceDynamic.SetScalarParameterValue` _dynamicmaterial_2 "BPTiling" _returnvalue_6)
          (`MaterialInstanceDynamic.SetScalarParameterValue` _dynamicmaterial_2 "BPtTilingDefault" 1.0)
          (else
            (`MaterialInstanceDynamic.SetScalarParameterValue` _dynamicmaterial_2 "BPTiling" 1.0)
            (`MaterialInstanceDynamic.SetScalarParameterValue` _dynamicmaterial_2 "BPtTilingDefault" _returnvalue_6))))
      (if (`self.SplineLoop`)
        (bind _returnvalue_13 (`AddComponent|NODE_AddSplineMeshComponent-8` :`bManualAttachment` true))
        (`SplineMeshComponent.SetSplineUpDir` _returnvalue_13 (`self.In Spline Up Dir`) true)
        (`StaticMeshComponent.SetStaticMesh` _returnvalue_13 (`self.MeshInstance`))
        (`SplineMeshComponent.SetStartScale` _returnvalue_13 (`KismetMathLibrary.MakeVector2D` _dynamicscalemesh_4 _dynamicscalemesh_4) true)
        (`SplineMeshComponent.SetEndScale` _returnvalue_13 (`KismetMathLibrary.MakeVector2D` _dynamicscalemesh_4 _dynamicscalemesh_4) true)
        (bind _output_get_3 (set `self.SplineMeshArray` _returnvalue_13))
        (`KismetArrayLibrary.Array_Add` (`self.MeshArray`) _output_get_3)
        (`SplineMeshComponent.SetStartScale` _returnvalue_13 (`KismetMathLibrary.MakeVector2D` _dynamicscalemesh_3 _dynamicscalemesh_3) true)
        (`SplineMeshComponent.SetEndScale` _returnvalue_13 (`KismetMathLibrary.MakeVector2D` _dynamicscalemesh_3 _dynamicscalemesh_3) true)
        (bind _returnvalue_14 (`PrimitiveComponent.CreateDynamicMaterialInstance` _returnvalue_13 0 (`self.MaterialInstance`) "None"))
        (bind _output_get_4 (set `self.DynamicMaterial` _returnvalue_14))
        (`KismetArrayLibrary.Array_Add` (`self.DynamicMaterialArray`) _output_get_4)
        (`PrimitiveComponent.SetMaterial` _returnvalue_13 0 _returnvalue_14)
        (bind _returnvalue_15 (* _index (`self.MeshDistanceScale(Type1`)))
        ;[0 1 0.491] SplineMeshTypeOne(SplineLoop
        (`SplineMeshComponent.SetStartAndEnd` _returnvalue_13 (`SplineComponent.GetLocationAtDistanceAlongSpline` _spline_2 _returnvalue_15 "World") (* (`SplineComponent.GetDirectionAtDistanceAlongSpline` _spline_2 _returnvalue_15 "World") _tangentscale_type1_3) (`SplineComponent.GetLocationAtDistanceAlongSpline` _spline_2 _returnvalue "World") (* (`SplineComponent.GetDirectionAtDistanceAlongSpline` _spline_2 _returnvalue "World") _tangentscale_type1_3) true)
        (`self.BPCommunicationMaterialUV` _returnvalue_15 _returnvalue _returnvalue (`self.DynamicMaterial`)) ; Communication module with material
        (`MaterialInstanceDynamic.SetScalarParameterValue` _dynamicmaterial_3 "BPSpeed" (`self.Speed`))
        (if (`self.TextureLoop`)
          (`MaterialInstanceDynamic.SetScalarParameterValue` _dynamicmaterial_3 "BPTiling" _returnvalue_7)
          (`MaterialInstanceDynamic.SetScalarParameterValue` _dynamicmaterial_3 "BPtTilingDefault" 1.0)
          (else
            (`MaterialInstanceDynamic.SetScalarParameterValue` _dynamicmaterial_3 "BPTiling" 1.0)
            (`MaterialInstanceDynamic.SetScalarParameterValue` _dynamicmaterial_3 "BPtTilingDefault" _returnvalue_7)))))
    (:`NewEnumerator1`
      (set `self.TypeTwo` true)
      (for _index_2 (range (+ (- _returnvalue_4 2) 1)) :!label _label
        (bind _returnvalue_16 (`AddComponent|NODE_AddSplineMeshComponent-7` :`bManualAttachment` true))
        (`SplineMeshComponent.SetSplineUpDir` _returnvalue_16 (`self.In Spline Up Dir`) true)
        (`StaticMeshComponent.SetStaticMesh` _returnvalue_16 (`self.MeshInstance`))
        (`SplineMeshComponent.SetStartScale` _returnvalue_16 (`KismetMathLibrary.MakeVector2D` _dynamicscalemesh_5 _dynamicscalemesh_5) true)
        (`SplineMeshComponent.SetEndScale` _returnvalue_16 (`KismetMathLibrary.MakeVector2D` _dynamicscalemesh_5 _dynamicscalemesh_5) true)
        (bind _output_get_5 (set `self.SplineMeshArray` _returnvalue_16))
        (`KismetArrayLibrary.Array_Add` (`self.MeshArray`) _output_get_5)
        (`SplineMeshComponent.SetStartScale` _returnvalue_16 (`KismetMathLibrary.MakeVector2D` _dynamicscalemesh_6 _dynamicscalemesh_6) true)
        (`SplineMeshComponent.SetEndScale` _returnvalue_16 (`KismetMathLibrary.MakeVector2D` _dynamicscalemesh_6 _dynamicscalemesh_6) true)
        (bind _returnvalue_17 (`PrimitiveComponent.CreateDynamicMaterialInstance` _returnvalue_16 0 (`self.MaterialInstance`) "None"))
        (bind _output_get_6 (set `self.DynamicMaterial` _returnvalue_17))
        (`KismetArrayLibrary.Array_Add` (`self.DynamicMaterialArray`) _output_get_6)
        (`PrimitiveComponent.SetMaterial` _returnvalue_16 0 _returnvalue_17)
        (if (`self.TypeTwo`)
          (bind (_location _tangent) (`SplineComponent.GetLocationAndTangentAtSplinePoint` _spline_3 _index_2 "World"))
          (bind _returnvalue_18 (+ _index_2 1))
          (bind (_location_2 _tangent_2) (`SplineComponent.GetLocationAndTangentAtSplinePoint` _spline_3 _returnvalue_18 "World"))
          ;[0.9536 1 0] SplineMeshTypeTwo(Fully fit the tangent of spline, and the material is stretched unevenly with the tangent
          (`SplineMeshComponent.SetStartAndEnd` _returnvalue_16 _location _tangent _location_2 _tangent_2 true)
          (else
            ;[1 0 0.01872] SplineMeshTypeThree(Tangents that do not fully fit the spline automatically generate equal controllable scaling tangents, and the material is stretched evenly with the tangents
            (`SplineMeshComponent.SetStartAndEnd` _returnvalue_16 _location (* (`SplineComponent.GetDirectionAtSplinePoint` _spline_3 _index_2 "World") _tangentscale_type1_3_3) _location_2 (* (`SplineComponent.GetDirectionAtSplinePoint` _spline_3 _returnvalue_18 "World") _tangentscale_type1_3_3) true)))
        (`self.BPCommunicationMaterialUV` (`SplineComponent.GetDistanceAlongSplineAtSplinePoint` _spline_3 _index_2) (`SplineComponent.GetDistanceAlongSplineAtSplinePoint` _spline_3 _returnvalue_18) _returnvalue_5 (`self.DynamicMaterial`)) ; Communication module with material
        (`MaterialInstanceDynamic.SetScalarParameterValue` _dynamicmaterial "BPSpeed" (`self.Speed`))
        (if (`self.TextureLoop`)
          (`MaterialInstanceDynamic.SetScalarParameterValue` _dynamicmaterial "BPTiling" _returnvalue_8)
          (`MaterialInstanceDynamic.SetScalarParameterValue` _dynamicmaterial "BPtTilingDefault" 1.0)
          (else
            (`MaterialInstanceDynamic.SetScalarParameterValue` _dynamicmaterial "BPTiling" 1.0)
            (`MaterialInstanceDynamic.SetScalarParameterValue` _dynamicmaterial "BPtTilingDefault" _returnvalue_8)))))
    (:`NewEnumerator2`
      (set `self.TypeTwo` false)
      (goto _label))))